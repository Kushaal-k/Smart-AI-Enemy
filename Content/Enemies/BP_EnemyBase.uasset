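; Base enemy character that provides sword combat actions, a patrol route getter and tiered movement speeds.
; Attack, wield and sheath events play montages, then fire dispatchers for their end, with attack also firing on interruption.
; Montage notifies time spawning the sword onto the right-hand socket and destroying it, updating the wielding flag.
; SetMovementSpeed maps an idle-to-sprint enum to the character's max walk speed.
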(event `Attack`
  ;[1 1 1] Default Attack
  (`|PlayMontage` (`self.Mesh`) "/Game/Assets/animation/Montages/Montage_Sword_Sheild_Slash.Montage_Sword_Sheild_Slash"
    (:`OnCompleted`
      _)
    (:`OnInterrupted`
      _))
  (`self.OnAttackEnd`))

(event `WieldSword`
  ;[1 1 1] Sword Wield
  (bind _notifyname (`|PlayMontage` (`self.Mesh`) "/Game/Assets/animation/Montages/Montage_Sword_Draw.Montage_Sword_Draw")
    (:`OnCompleted`
      (`self.OnWieldSword`))
    (:`OnNotifyBegin`
      (switch `name` _notifyname
        (:`HoldSword`
          (bind _returnvalue (`|SpawnActorFromClass` "/Game/Weapons/BP_Sword.BP_Sword_C" (`self.GetTransform`) "Undefined" "MultiplyWithRoot" null null))
          (bind _output_get (set `self.SwordActor` _returnvalue))
          (`self.K2_AttachToComponent` _output_get (`self.Mesh`) "hand_r_sword_socket" "SnapToTarget" "SnapToTarget" "SnapToTarget" true)
          (set `self.IsWieldingSword` true))))))

(event `SheathSword`
  ;[1 1 1] Sheath Sword
  (bind _notifyname (`|PlayMontage` (`self.Mesh`) "/Game/Assets/animation/Montages/Montage_Shealting_Sword.Montage_Shealting_Sword")
    (:`OnCompleted`
      (`self.OnSheathSword`))
    (:`OnNotifyBegin`
      (switch `name` _notifyname
        (:`DropSword`
          (`self.K2_DestroyActor` (`self.SwordActor`))
          (set `self.IsWieldingSword` false))))))

(fn `GetPatrolRoute`
  (returns (PatrolRoute :type "/Game/Enemies/AI/BP_PatrolRoute Object Reference"))
  (return (`self.PatrolRoute`)))

(fn `SetMovementSpeed`
  (params (Speed :type "/Game/Enemies/AI/Enums/E_MovementSpeed Enum" :default "NewEnumerator0"))
  (returns (SpeedValue :type "Float (double-precision)"))
  (bind _output_get (set `CharacterMovementComponent.MaxWalkSpeed` (select `/Game/Enemies/AI/Enums/E_MovementSpeed` Speed :`NewEnumerator1` 100.0 :`NewEnumerator2` 300.0 :`NewEnumerator3` 500.0) (`self.CharacterMovement`)))
  (return _output_get))

(fn `UserConstructionScript`)